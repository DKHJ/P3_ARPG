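; AI controller for the melee enemy that starts its behavior tree on possession and handles first detection of the player.
; When AI Perception successfully senses a Player-tagged actor and the pawn is not yet alerted, it flags the player as detected and fills the blackboard's alert, line-of-sight and target keys.
; It also marks the pawn alerted and stores the player reference on it; losing sight is not handled here.
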(event `self.ReceivePossess`
  (params (PossessedPawn :type "Pawn Object Reference"))
  (`self.RunBehaviorTree` "/Game/AI/BT_MeleeEnemy.BT_MeleeEnemy"))

(event `self.AIPerception.OnTargetPerceptionUpdated`
  (params (Actor :type "Actor Object Reference") (Stimulus :type "AIStimulus Structure"))
  (bind _blackboard (`self.Blackboard`))
  (if (and (`self.ActorHasTag` Actor "Player") (`.bSuccessfullySensed` (break `AIStimulus` Stimulus)))
    (bind _asplayer_character (cast `/Game/Characters/ThirdPerson/PlayerCharacter` Actor))
    (bind _asbp_melee_enemy (cast `/Game/AI/BP_MeleeEnemy` (`self.K2_GetPawn`)))
    (if (not (`/Game/AI/BP_MeleeEnemy.IsAlerted?` _asbp_melee_enemy))
      (set `/Game/Characters/ThirdPerson/PlayerCharacter.IsDetected?` true _asplayer_character)
      (`BlackboardComponent.SetValueAsBool` _blackboard (`self.Alerted?`) true)
      (`BlackboardComponent.SetValueAsBool` _blackboard (`self.HasLineOfSight?`) true)
      (`BlackboardComponent.SetValueAsObject` _blackboard (`self.OtherActor`) Actor)
      (bind _asbp_melee_enemy_2 (cast `/Game/AI/BP_MeleeEnemy` (`self.K2_GetPawn`)))
      (set `/Game/AI/BP_MeleeEnemy.IsAlerted?` true _asbp_melee_enemy_2)
      (set `/Game/AI/BP_MeleeEnemy.PlayerReference` _asplayer_character _asbp_melee_enemy_2))))

(fn `UserConstructionScript`)
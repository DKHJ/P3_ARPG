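; Melee enemy character that damages the player when its weapon sphere overlaps the player's mesh.
; TakeDamage lowers health and calls SetDeath at zero, which ragdolls the body, spawns a selected boss limb and a health pickup, and removes the widget.
; Corpses become useable with a custom-depth outline and "Loot Enemy" prompt, though using them does nothing.
; It registers itself in GroupArray; SetAlerted is empty and health bar updating is unwired.
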(event `self.ReceiveBeginPlay`
  (`KismetArrayLibrary.Array_AddUnique` (`self.GroupArray`) self))

(event `self.WeaponCollisionSphere.OnComponentBeginOverlap`
  (params (OverlappedComponent :type "PrimitiveComponent Object Reference") (OtherActor :type "Actor Object Reference") (OtherComp :type "PrimitiveComponent Object Reference") (OtherBodyIndex :type Integer) (bFromSweep :type Boolean) (SweepResult :type "HitResult Structure (by ref)"))
  (bind _asplayer_character (cast `/Game/Characters/ThirdPerson/PlayerCharacter` OtherActor))
  (if (== OtherComp (`Character.Mesh` _asplayer_character))
    (`/Game/Characters/ThirdPerson/PlayerCharacter.TakeDamage` _asplayer_character (`self.DamageAmount`))))

(fn `BeginOutlineFocus`
  (returns (Success :type Boolean))
  (`PrimitiveComponent.SetRenderCustomDepth` (`self.Mesh`) true)
  (return true))

(fn `EndOutlineFocus`
  (returns (Success :type Boolean))
  (`PrimitiveComponent.SetRenderCustomDepth` (`self.Mesh`) false)
  (return true))

(fn `GetActorUseable`
  (returns (Success :type Boolean))
  (return (`self.IsUseable`)))

(fn `GetIsAlerted`
  (returns (`IsAlerted??` :type Boolean))
  (return (`self.IsAlerted?`)))

(fn `GetUseActionText`
  (returns (ActionText :type Text))
  (return "Loot Enemy"))

(fn `IsAlive`
  (returns (Return :type Boolean))
  (return (>= (`self.Health`) 0.0)))

(fn `OnActorUsed`
  (params (Controller :type "PlayerController Object Reference"))
  (returns (Success :type Boolean))
  (return false))

(fn `SetAlerted`)

(fn `SetDeath`
  (`CharacterMovementComponent.DisableMovement` (`self.CharacterMovement`))
  (`PrimitiveComponent.SetCollisionEnabled` (`self.Mesh`) "QueryAndPhysics")
  (`PrimitiveComponent.SetSimulatePhysics` (`self.Mesh`) true)
  (`PrimitiveComponent.SetCollisionEnabled` (`self.CapsuleComponent`) "NoCollision")
  (set `self.IsUseable` true)
  (`self.SpawnBossItem`)
  (`/Engine/EditorBlueprintResources/StandardMacros.DoOnce` false
    (:`Completed`
      (`|SpawnActorFromClass` "/Game/Blueprints/PickUps/BP_HealthPickUp.BP_HealthPickUp_C" (`KismetMathLibrary.MakeTransform` (+ (`self.K2_GetActorLocation`) (0.0 0.0 10.0))) "AdjustIfPossibleButAlwaysSpawn" "OverrideRootScale" null null)
      (`ActorComponent.K2_DestroyComponent` (`self.Widget`)))))

(fn `SpawnBossItem`
  (bind (_returnvalue_location _returnvalue_rotation _returnvalue_scale) (`KismetMathLibrary.BreakTransform` (`self.GetTransform`)))
  (switch `/Game/AI/MeleeEnemy/BossDropItems` (`self.BossItemDrop`)
    (:`NewEnumerator0`
      (`|SpawnActorFromClass` "/Game/Blueprints/PickUps/BP_BossArmL.BP_BossArmL_C" (`KismetMathLibrary.MakeTransform` (+ _returnvalue_location (0.0 0.0 0.0)) _returnvalue_rotation _returnvalue_scale) "Undefined" "OverrideRootScale" null null))
    (:`NewEnumerator1`
      (`|SpawnActorFromClass` "/Game/Blueprints/PickUps/BP_BossArmR.BP_BossArmR_C" (`self.GetTransform`) "Undefined" "OverrideRootScale" null null))
    (:`NewEnumerator2`
      (`|SpawnActorFromClass` "/Game/Blueprints/PickUps/BP_BossLegL.BP_BossLegL_C" (`self.GetTransform`) "Undefined" "OverrideRootScale" null null))
    (:`NewEnumerator3`
      (`|SpawnActorFromClass` "/Game/Blueprints/PickUps/BP_BossLegR.BP_BossLegR_C" (`self.GetTransform`) "Undefined" "OverrideRootScale" null null))))

(fn `TakeDamage`
  (params (`Incoming Damage` :type "Float (double-precision)"))
  (bind _output_get (set `self.Health` (- (`self.Health`) `Incoming Damage`)))
  (if (<= _output_get 0.0)
    (`self.SetDeath`)
    (else
      (`KismetSystemLibrary.PrintString` (`KismetStringLibrary.Concat_StrStr` "Enemy Health: " (`KismetStringLibrary.Conv_DoubleToString` _output_get)) true true (struct :`R` 1.0 :`G` 0.055564 :`A` 1.0)))))

(fn `UpdateWalkSpeed`
  (params (`New Walk Speed` :type "Float (double-precision)"))
  (set `CharacterMovementComponent.MaxWalkSpeed` `New Walk Speed` (`self.CharacterMovement`)))

(fn `UserConstructionScript`)
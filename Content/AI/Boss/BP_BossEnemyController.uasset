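; AI controller for the boss enemy that runs its behavior tree and reacts to spotting the player.
; On possess it sets up the BB_BossEnemy blackboard and starts BT_BossEnemy.
; Successful perception of a Player-tagged actor marks the player as detected, writes line-of-sight and actor keys to the blackboard, and stores the player reference on the boss pawn.
; Lost perception is not handled, so nothing here clears that state.
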(event `self.ReceivePossess`
  (params (PossessedPawn :type "Pawn Object Reference"))
  (`self.UseBlackboard` "/Game/AI/Boss/BB_BossEnemy.BB_BossEnemy")
  (`self.RunBehaviorTree` "/Game/AI/Boss/BT_BossEnemy.BT_BossEnemy"))

(event `self.AIPerception.OnTargetPerceptionUpdated`
  (params (Actor :type "Actor Object Reference") (Stimulus :type "AIStimulus Structure"))
  (bind _blackboard (`self.Blackboard`))
  (if (and (`self.ActorHasTag` Actor "Player") (`.bSuccessfullySensed` (break `AIStimulus` Stimulus)))
    (bind _asplayer_character (cast `/Game/Characters/ThirdPerson/PlayerCharacter` Actor))
    (cast `/Game/AI/Boss/BP_BossEnemy` (`self.K2_GetPawn`))
    (set `/Game/Characters/ThirdPerson/PlayerCharacter.IsDetected?` true _asplayer_character)
    (`BlackboardComponent.SetValueAsBool` _blackboard (`self.HasLineOfSight?`) true)
    (`BlackboardComponent.SetValueAsObject` _blackboard (`self.OtherActor`) null)
    (bind _asbp_boss_enemy (cast `/Game/AI/Boss/BP_BossEnemy` (`self.K2_GetPawn`)))
    (set `/Game/AI/Boss/BP_BossEnemy.PlayerReference` _asplayer_character _asbp_boss_enemy)))

(fn `UserConstructionScript`)
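; BP_BossEnemy is a boss enemy that damages the player and tracks its own health.
; Scratch and left/right slam overlap events apply scratch or slam damage when they hit the player character's mesh, with both slams sharing one damage path.
; TakeDamage subtracts health and prints what remains, or calls SetDeath at zero, which destroys the boss and calls ResetLevel on the player.
; Helper functions expose an alive check and set walk speed.
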(event `self.ScratchSphere.OnComponentBeginOverlap`
  (params (OverlappedComponent :type "PrimitiveComponent Object Reference") (OtherActor :type "Actor Object Reference") (OtherComp :type "PrimitiveComponent Object Reference") (OtherBodyIndex :type Integer) (bFromSweep :type Boolean) (SweepResult :type "HitResult Structure (by ref)"))
  (bind _asplayer_character (cast `/Game/Characters/ThirdPerson/PlayerCharacter` OtherActor))
  (if (== OtherComp (`Character.Mesh` _asplayer_character))
    (`/Game/Characters/ThirdPerson/PlayerCharacter.TakeDamage` _asplayer_character (`self.ScratchDamage`))))

(event `self.LeftSlam.OnComponentBeginOverlap`
  (params (OverlappedComponent :type "PrimitiveComponent Object Reference") (OtherActor :type "Actor Object Reference") (OtherComp :type "PrimitiveComponent Object Reference") (OtherBodyIndex :type Integer) (bFromSweep :type Boolean) (SweepResult :type "HitResult Structure (by ref)"))
  (bind _asplayer_character (cast `/Game/Characters/ThirdPerson/PlayerCharacter` (stale `self.RightSlam.OnComponentBeginOverlap` OtherActor) :!label _label))
  (if (== (stale `self.RightSlam.OnComponentBeginOverlap` OtherComp) (`Character.Mesh` _asplayer_character))
    (`/Game/Characters/ThirdPerson/PlayerCharacter.TakeDamage` _asplayer_character (`self.SlamDamage`))))

(event `self.RightSlam.OnComponentBeginOverlap`
  (params (OverlappedComponent :type "PrimitiveComponent Object Reference") (OtherActor :type "Actor Object Reference") (OtherComp :type "PrimitiveComponent Object Reference") (OtherBodyIndex :type Integer) (bFromSweep :type Boolean) (SweepResult :type "HitResult Structure (by ref)"))
  (goto _label))

(fn `IsAlive`
  (returns (Return :type Boolean))
  (return (> (`self.Health`) 0.0)))

(fn `SetDeath`
  (`self.K2_DestroyActor`)
  (bind _asplayer_character (cast `/Game/Characters/ThirdPerson/PlayerCharacter` (`GameplayStatics.GetPlayerCharacter` 0)))
  (`/Game/Characters/ThirdPerson/PlayerCharacter.ResetLevel` _asplayer_character))

(fn `TakeDamage`
  (params (IncomingDamage :type "Float (double-precision)"))
  (bind _output_get (set `self.Health` (- (`self.Health`) IncomingDamage)))
  (if (<= _output_get 0.0)
    (`self.SetDeath`)
    (else
      (`KismetSystemLibrary.PrintString` (`KismetStringLibrary.Concat_StrStr` "Boss Health: " (`KismetStringLibrary.Conv_DoubleToString` _output_get)) true true (struct :`R` 1.0 :`G` 0.055564 :`A` 1.0)))))

(fn `UpdateWalkSpeed`
  (params (`New Walk Speed` :type "Float (double-precision)"))
  (set `CharacterMovementComponent.MaxWalkSpeed` `New Walk Speed` (`self.CharacterMovement`)))

(fn `UserConstructionScript`)
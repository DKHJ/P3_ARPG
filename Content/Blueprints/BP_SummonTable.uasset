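; BP_SummonTable is a table actor that enables boss summoning through the game instance.
; When the player overlaps its Box, it flags OverlappingSummonTable on the PlayerCharacter.
; If the game instance's SetTheTable flag is true, it reveals the LeftLeg component and sets CanSummonBoss on the game instance.
; It has no end-overlap handling, so it never clears these flags itself.
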(event `self.Box.OnComponentBeginOverlap`
  (params (OverlappedComponent :type "PrimitiveComponent Object Reference") (OtherActor :type "Actor Object Reference") (OtherComp :type "PrimitiveComponent Object Reference") (OtherBodyIndex :type Integer) (bFromSweep :type Boolean) (SweepResult :type "HitResult Structure (by ref)"))
  (bind _asplayer_character (cast `/Game/Characters/ThirdPerson/PlayerCharacter` OtherActor))
  (set `/Game/Characters/ThirdPerson/PlayerCharacter.OverlappingSummonTable?` true _asplayer_character)
  (bind _asbp_game_instance (cast `/Game/Blueprints/Game/BP_GameInstance` (`GameplayStatics.GetGameInstance`)))
  (if (`/Game/Blueprints/Game/BP_GameInstance.SetTheTable?` _asbp_game_instance)
    (`SceneComponent.SetVisibility` (`self.LeftLeg`) true false)
    (bind _asbp_game_instance_2 (cast `/Game/Blueprints/Game/BP_GameInstance` (`GameplayStatics.GetGameInstance`)))
    (set `/Game/Blueprints/Game/BP_GameInstance.CanSummonBoss?` true _asbp_game_instance_2)))

(fn `UserConstructionScript`)
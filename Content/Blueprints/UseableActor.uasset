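; UseableActor is an interactable actor with a static mesh that can be highlighted and used by a controller.
; Focus functions toggle the mesh's custom depth rendering, the usual hook for a post-process outline.
; It reports its useable flag and builds prompt text from its action and name.
; OnActorUsed is a stub returning false, and the event graph and construction script are empty.
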(fn `BeginOutlineFocus`
  (returns (Success :type Boolean))
  (`PrimitiveComponent.SetRenderCustomDepth` (`self.StaticMesh`) true)
  (return true))

(fn `EndOutlineFocus`
  (returns (Success :type Boolean))
  (`PrimitiveComponent.SetRenderCustomDepth` (`self.StaticMesh`) false)
  (return true))

(fn `GetActorUseable`
  (returns (Success :type Boolean))
  (return (`self.IsUseable`)))

(fn `GetUseActionText`
  (returns (ActionText :type Text))
  (return (`|FormatText` "{action} {name}" (`self.Action`) (`KismetTextLibrary.Conv_NameToText` (`self.Name`)))))

(fn `OnActorUsed`
  (params (Controller :type "PlayerController Object Reference"))
  (returns (Success :type Boolean))
  (return false))

(fn `UserConstructionScript`)
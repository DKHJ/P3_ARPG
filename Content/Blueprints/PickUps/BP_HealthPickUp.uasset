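; BP_HealthPickUp is a health pickup actor that flies to the player on its own and then destroys itself.
; After a short random delay from BeginPlay, it stops physics simulation on Sphere1 and stores its current location.
; A timeline then lerps it from that location to player 0's live position, so it tracks movement without overlap checks.
; FinishPickUpItem only destroys the actor; no health is granted here.
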(event `self.ReceiveBeginPlay`
  (`KismetSystemLibrary.Delay` (`KismetMathLibrary.RandomFloatInRange` 0.5 1.0))
  (`PrimitiveComponent.SetSimulatePhysics` (`self.Sphere1`) false)
  (set `self.IntialActorLocation` (`self.K2_GetActorLocation`))
  (bind (_direction _newtrack_0) (`Timeline|Timeline_0`)
    (:`Update`
      (`self.K2_SetActorLocation` (`KismetMathLibrary.VLerp` (`self.IntialActorLocation`) (`self.K2_GetActorLocation` (`GameplayStatics.GetPlayerCharacter` 0)) _newtrack_0)))
    (:`Finished`
      (`self.FinishPickUpItem`))))

(event `FinishPickUpItem`
  (`self.K2_DestroyActor`))

(fn `UserConstructionScript`)
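; BP_BreakablePot is a destructible pot actor that drops a health pickup when broken.
; TakeDamage subtracts incoming damage from Health and calls DestroyPot once it reaches zero or below.
; DestroyPot plays a 2D break sound, removes the particle component, spawns BP_HealthPickUp at the mesh's location and destroys the actor.
; The event graph and construction script hold no logic.
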(fn `DestroyPot`
  (`GameplayStatics.PlaySound2D` "/Game/Audio/BreakPot.BreakPot" 1.0 1.0 0.0 null null)
  (`ActorComponent.K2_DestroyComponent` (`self.ParticleSystem`))
  (`|SpawnActorFromClass` "/Game/Blueprints/PickUps/BP_HealthPickUp.BP_HealthPickUp_C" (`KismetMathLibrary.Conv_VectorToTransform` (`SceneComponent.K2_GetComponentLocation` (`self.StaticMesh`))) "Undefined" "OverrideRootScale" null null)
  (`self.K2_DestroyActor`))

(fn `TakeDamage`
  (params (IncomingDamage :type "Float (double-precision)"))
  (bind _output_get (set `self.Health` (- (`self.Health`) IncomingDamage)))
  (if (<= _output_get 0.0)
    (`self.DestroyPot`)))

(fn `UserConstructionScript`)